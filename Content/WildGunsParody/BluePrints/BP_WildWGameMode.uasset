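; BP_WildWGameMode is the game mode Blueprint for the WildGunsParody game, handling a start-up sound and a timer.
; BeginPlay plays a 2D sound and sets an event timer using the Time variable, while a TimeEvent event prints a "WAZAA" debug string.
; Tick sets RemainTime to Time minus the frame's delta, so the value does not accumulate into a countdown.
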(event Custom|TimeEvent
  (Development|PrintString "WAZAA"))

(event EventBeginPlay
  (Audio|PlaySound2D (Variables|Default|GetSound) 1.0 1.0 0.0 0 0)
  (Utilities|Time|SetTimerbyEvent (EventDispatchers|CreateEvent :!event Custom|TimeEvent) (Variables|Default|GetTime)))

(event EventTick
  (params (DeltaSeconds :type Float%20%28single-precision%29))
  (Variables|Default|SetremainTime (- (Variables|Default|GetTime) DeltaSeconds)))

(fn ConstructionScript)