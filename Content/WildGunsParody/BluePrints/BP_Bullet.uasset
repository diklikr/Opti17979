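; BP_Bullet is a projectile actor that hides itself on impact or after a timed lifetime instead of being destroyed.
; ShootBullet rebinds the projectile movement to the collision component, re-enables simulation and sets velocity along the given direction.
; On hit, it takes a BP_DecalBullet from the game mode's decal pool, cached at BeginPlay, and sets it up as a fading impact decal.
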(event OnComponentHit(collision)
  (params (HitComponent :type Primitive%20Component%20Object%20Reference) (OtherActor :type Actor%20Object%20Reference) (OtherComp :type Primitive%20Component%20Object%20Reference) (NormalImpulse :type Vector :default "0, 0, 0") (Hit :type Hit%20Result%20Structure%20%28by%20ref%29))
  ;[0.15 0.15 0.15 0.5] Collision
  (Development|PrintString (Utilities|GetDisplayName OtherActor))
  (bind _returnvalue (Class|ActorPool|GetActorfromPool (Variables|Default|GetDecal%20Pool%20local)))
  (bind _asbp_decal_bullet (Utilities|Casting|CastToBP_DecalBullet _returnvalue))
  (Rendering|Components|Decal|SetFadeIn (Variables|/Script/Engine.DecalActor|GetDecal _asbp_decal_bullet) 0.0 0.0)
  (Class|DecalimpactBullet|SetupDecal _asbp_decal_bullet Hit 2.0 1.0)
  (Class|ActorUtilities|ToggleActorHidden self true))

(event Custom|Lifetime
  (params (lifetime :type Float%20%28double-precision%29))
  ;[0.15 0.15 0.15 0.5] LifeTime
  (Utilities|FlowControl|Delay lifetime)
  (Class|ActorUtilities|ToggleActorHidden self true))

(event Custom|ShootBullet
  (params (Direction :type Vector))
  (bind _projectilemovement (Variables|Default|GetProjectileMovement))
  ;[0.15 0.15 0.15 0.5] ShootBullet
  (Development|PrintString "Shoot")
  ;;[0.15 0.15 0.15 0.5] CRITICAL
  (Components|Movement|SetUpdatedComponent (Variables|Default|GetProjectileMovement) (Variables|Default|Getcollision))
  (Variables|/Script/Engine.ProjectileMovementComponent|SetbSimulationEnabled _projectilemovement true)
  (Variables|/Script/Engine.MovementComponent|SetVelocity _projectilemovement (* Direction (Variables|Default|GetprojectileSpeed))))

(event EventBeginPlay
  ;[0.15 0.15 0.15 0.5] BeginPlay
  (bind _asbp_wild_wgame_mode (Utilities|Casting|CastToBP_WildWGameMode (Game|GetGameMode)))
  (Variables|Default|SetDecal%20Pool%20local (Variables|/Game/WildGunsParody/BluePrints/BP_WildWGameMode.BP_WildWGameMode_C|GetDecalPool _asbp_wild_wgame_mode)))

(event Collision|EventActorBeginOverlap
  (params (OtherActor :type Actor%20Object%20Reference)))

(event EventTick
  (params (DeltaSeconds :type Float%20%28single-precision%29)))

(fn ConstructionScript)