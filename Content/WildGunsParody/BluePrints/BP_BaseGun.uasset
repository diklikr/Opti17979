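; Base gun Blueprint for WildGunsParody that fires pooled bullets from its muzzle toward the mouse cursor.
; Shoot takes an actor from BulletPool, unhides it, moves it to the muzzle, launches it and passes ShootDelay to its Lifetime.
; MouseRaycast traces from the camera through the deprojected cursor and returns the muzzle-to-hit direction, or muzzle-to-trace-end on a miss.
; CanShoots gates firing and resets after the Lifetime call, but stays false if the bullet cast fails.
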(event EventBeginPlay)

(event Collision|EventActorBeginOverlap
  (params (OtherActor :type Actor%20Object%20Reference)))

(event EventTick
  (params (DeltaSeconds :type Float%20%28single-precision%29)))

(fn ConstructionScript)

(fn Shoot
  (if (Variables|Default|GetcanShoots)
    (Variables|Default|SetcanShoots false)
    (bind _returnvalue (Class|ActorPool|GetActorfromPool (Variables|Default|GetBulletPool)))
    (Rendering|SetActorHiddenInGame _returnvalue false)
    (bind _asbp_bullet (Utilities|Casting|CastToBP_Bullet _returnvalue)
      (:then
        (Transformation|SetActorLocation _asbp_bullet (Transformation|GetWorldLocation (Variables|Default|GetMuzzle)) false false)
        (bind _point (CallFunction|MouseRaycast))
        (Default|ShootBullet _asbp_bullet _point)
        (Default|Lifetime _asbp_bullet (Variables|Default|GetShoot%20Delay))
        (Variables|Default|SetcanShoots true))
      (:CastFailed
        (Development|PrintString "cast not valid")))))

(fn MouseRaycast
  (bind _returnvalue (Game|GetPlayerController 0))
  (bind _muzzle (Variables|Default|GetMuzzle))
  (bind (_locationx _locationy) (Game|Player|GetMousePosition _returnvalue))
  (bind _returnvalue_2 (Transformation|GetWorldLocation _muzzle))
  (Variables|/Script/Engine.PlayerController|SetbShowMouseCursor _returnvalue true)
  (Variables|Default|SetstartPoint (Camera|GetCameraLocation (Variables|/Script/Engine.PlayerController|GetPlayerCameraManager _returnvalue)))
  (bind (_outhit _returnvalue_3) (Collision|LineTraceByChannel (Variables|Default|GetstartPoint) (+ (* (Math|Vector|Normalize (- (.WorldPosition (Class|GameplayStatics|DeprojectScreentoWorld _returnvalue (Math|Vector2D|MakeVector2D _locationx _locationy))) (Variables|Default|GetstartPoint))) (Variables|Default|GetdefaultRange)) (Variables|Default|GetstartPoint)) "TraceTypeQuery1" false 0 "None"))
  (if _returnvalue_3
    (return (Math|Vector|Normalize (- (.location _outhit) _returnvalue_2)))
    (else
      (return (Math|Vector|Normalize (- (.traceend _outhit) _returnvalue_2))))))