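; Enemy spawn point for the Wild Guns parody that places melee, moving and pop-up enemies at its own location.
; It caches BP_WildWGameMode on BeginPlay and exposes SpawnMelee, SpawnMove and SpawnPop events.
; Each event pulls an actor from the matching game mode pool instead of spawning one, unhides it, casts it and teleports it to the spawner without sweeping.
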(event Custom|SpawnMelee
  (bind _returnvalue (Class|ActorPool|GetActorfromPool (Variables|/Game/WildGunsParody/BluePrints/BP_WildWGameMode.BP_WildWGameMode_C|GetEnemyMeleePool (Variables|Default|GetAs%20BP%20Wild%20WGame%20Mode))))
  (Rendering|SetActorHiddenInGame _returnvalue false)
  (bind _asbp_enemy_melee (Utilities|Casting|CastToBP_EnemyMelee _returnvalue))
  (Transformation|SetActorLocation _asbp_enemy_melee (Transformation|GetActorLocation self) false false))

(event Custom|SpawnPop
  (bind _returnvalue (Class|ActorPool|GetActorfromPool (Variables|/Game/WildGunsParody/BluePrints/BP_WildWGameMode.BP_WildWGameMode_C|GetEnemyPool (Variables|Default|GetAs%20BP%20Wild%20WGame%20Mode))))
  (Rendering|SetActorHiddenInGame _returnvalue false)
  (bind _asbp_enemy_pop (Utilities|Casting|CastToBP_EnemyPop _returnvalue))
  (Transformation|SetActorLocation _asbp_enemy_pop (Transformation|GetActorLocation self) false false))

(event Custom|SpawnMove
  (bind _returnvalue (Class|ActorPool|GetActorfromPool (Variables|/Game/WildGunsParody/BluePrints/BP_WildWGameMode.BP_WildWGameMode_C|GetEnemyMovePool (Variables|Default|GetAs%20BP%20Wild%20WGame%20Mode))))
  (Rendering|SetActorHiddenInGame _returnvalue false)
  (bind _asbp_enemy_move (Utilities|Casting|CastToBP_EnemyMove _returnvalue))
  (Transformation|SetActorLocation _asbp_enemy_move (Transformation|GetActorLocation self) false false))

(event EventBeginPlay
  (bind _asbp_wild_wgame_mode (Utilities|Casting|CastToBP_WildWGameMode (Game|GetGameMode)))
  (Variables|Default|SetAs%20BP%20Wild%20WGame%20Mode _asbp_wild_wgame_mode))

(event Collision|EventActorBeginOverlap
  (params (OtherActor :type Actor%20Object%20Reference)))

(event EventTick
  (params (DeltaSeconds :type Float%20%28single-precision%29)))

(fn ConstructionScript)