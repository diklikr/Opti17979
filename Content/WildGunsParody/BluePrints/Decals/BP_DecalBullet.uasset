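; BP_DecalBullet is a bullet decal Blueprint that controls its visibility through an OpacityMask material parameter.
; On BeginPlay it creates a dynamic material instance from the decal and binds delegates for decal activation and fade start.
; ResetMat restores the mask to fully opaque, while TweenFade eases it from its current value to zero over a given duration using a float tween.
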(event Custom|ResetMat
  ;[0.15 0.15 0.15 0.5] Reset
  (Rendering|Material|SetScalarParameterValue (Variables|Default|GetRuntimeMat) (Variables|Default|GetOpacity%20Mask) 1.0 :!class /Script/Engine.MaterialInstanceDynamic))

(event Custom|TweenFade
  (params (Duration :type Float%20%28double-precision%29))
  (bind _returnvalue (Rendering|Material|GetScalarParameterValue (Variables|Default|GetRuntimeMat) (Variables|Default|GetOpacity%20Mask) :!class /Script/Engine.MaterialInstanceDynamic))
  (bind _value (|TweenFloat _returnvalue 0.0 Duration "InOutQuad")
    (:ApplyEasing
      (Rendering|Material|SetScalarParameterValue (Variables|Default|GetRuntimeMat) (Variables|Default|GetOpacity%20Mask) _value :!class /Script/Engine.MaterialInstanceDynamic))))

(event Custom|OnDecalActivated_Event)

(event Custom|OnDecalStartFade_Event
  (params (FadeDuration :type Float%20%28single-precision%29)))

(event EventBeginPlay
  (bind _returnvalue (Rendering|Material|CreateDynamicMaterialInstance (Variables|Default|GetDecal) :!class /Script/Engine.DecalComponent))
  (Variables|Default|SetRuntimeMat _returnvalue)
  (EventDispatchers|BindEventtoOnDecalActivated (EventDispatchers|CreateEvent :!event Custom|ResetMat))
  (EventDispatchers|BindEventtoOnDecalStartFade (EventDispatchers|CreateEvent :!event Custom|TweenFade)))

(event EventTick
  (params (DeltaSeconds :type Float%20%28single-precision%29)))

(fn ConstructionScript)