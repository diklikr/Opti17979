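; BP_EnemyMove is a movable enemy that travels to a destination assigned to it.
; SetDestination stores a target vector and a separate X position, then calls Move.
; Move runs AI MoveTo using the stored X with the target's Y and Z and a loose acceptance radius.
; On success it calls ToggleActorHidden to hide itself.
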(event Custom|SetDestination
  (params (TargetDest :type Vector) (TargetX :type Float%20%28double-precision%29))
  (bind _output_get (Variables|Default|SetDestination TargetDest))
  (Variables|Default|SetXpos TargetX)
  (CallFunction|Move _output_get))

(event EventBeginPlay
  (|CallParentFunction) ; This node is disabled and will not be called.\nDrag off pins to build functionality.
)

(event Collision|EventActorBeginOverlap
  (params (OtherActor :type Actor%20Object%20Reference))
  (|CallParentFunction OtherActor) ; This node is disabled and will not be called.\nDrag off pins to build functionality.
)

(event EventTick
  (params (DeltaSeconds :type Float%20%28single-precision%29))
  (|CallParentFunction DeltaSeconds) ; This node is disabled and will not be called.\nDrag off pins to build functionality.
)

(event EventMove
  (params (Destination :type Vector :default "0, 0, 0"))
  (bind _self self)
  (AI|AIMoveTo _self (Math|Vector|MakeVector (Variables|Default|GetXpos) (.y Destination) (.z Destination)) 0 2e+02 false
    (:OnSuccess
      (Class|ActorUtilities|ToggleActorHidden _self true))))

(fn ConstructionScript
  (|CallParentFunction))