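; Enemy for a Wild Guns parody that shoots at the player, moves on command and can spawn a power-up.
; On BeginPlay it takes the game mode's slow-bullet pool, then fires a pooled bullet toward the player on a self-repeating delay, skipped for BP_EnemyMelee.
; AI moves signal completion on success or failure alike.
; Taking damage plays a sound and hides the actor.
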(event Custom|ShootPlayer
  ;[0.15 0.15 0.15 0.5] ShootPlayer
  (if (not (== (Utilities|GetClass self) "/Game/WildGunsParody/BluePrints/Enemys/BP_EnemyMelee.BP_EnemyMelee_C"))
    (bind _returnvalue (Class|ActorPool|GetActorfromPool (Variables|Default|GetBullet%20Pool)))
    (bind _asbp_bullet (Utilities|Casting|CastToBP_Bullet _returnvalue))
    (Rendering|SetActorHiddenInGame _asbp_bullet false)
    (Transformation|SetActorLocation _asbp_bullet (Transformation|GetWorldLocation (Variables|Default|GetFirePoint)) false false)
    (Default|ShootBullet _asbp_bullet (Math|Vector|Normalize (- (Transformation|GetActorLocation (Game|Player|GetPlayerPawn 0)) (Transformation|GetActorLocation))))
    (Default|Lifetime _asbp_bullet 3e+01)
    (Utilities|FlowControl|Delay 3.0)
    (CallFunction|ShootPlayer)))

(event Custom|Move
  (params (Destination :type Vector))
  ;[0.15 0.15 0.15 0.5] Move
  (AI|AIMoveTo self (Math|Vector|MakeVector 0.0 (.y Destination) (.z Destination)) 0 5e+02 false
    (:OnSuccess
      _)
    (:OnFail
      _))
  (Default|CallOnFinishMove))

(event Custom|PowerUpSpawn
  ;[0.15 0.15 0.15 0.5] PowerUP
  (Game|SpawnActorfromClass (Variables|Default|GetPowerUP) (Transformation|GetActorTransform self) "Undefined" "MultiplyWithRoot" 0 0))

(event EventBeginPlay
  ;[0.15 0.15 0.15 0.5] BeginPlay
  (|CallParentFunction)
  (bind _asbp_wild_wgame_mode (Utilities|Casting|CastToBP_WildWGameMode (Game|GetGameMode)))
  (Variables|Default|SetBullet%20Pool (Variables|/Game/WildGunsParody/BluePrints/BP_WildWGameMode.BP_WildWGameMode_C|GetBulletSlowPool _asbp_wild_wgame_mode))
  (CallFunction|ShootPlayer))

(event Collision|EventActorBeginOverlap
  (params (OtherActor :type Actor%20Object%20Reference))
  (|CallParentFunction OtherActor) ; This node is disabled and will not be called.\nDrag off pins to build functionality.
)

(event EventTick
  (params (DeltaSeconds :type Float%20%28single-precision%29))
  (|CallParentFunction DeltaSeconds) ; This node is disabled and will not be called.\nDrag off pins to build functionality.
)

(event EventTakeDamage
  (params (damage :type Float%20%28double-precision%29))
  ;[0.15 0.15 0.15 0.5] TakeDamage
  (|CallParentFunction damage)
  (Audio|PlaySound2D (Variables|Default|GetSound) 1.0 1.0 0.0 0 0)
  (Class|ActorUtilities|ToggleActorHidden self true))

(fn ConstructionScript
  (|CallParentFunction))