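; BP_EnemyPop is an enemy-related Blueprint in WildGunsParody that spawns another actor whenever it takes damage.
; Its TakeDamage event spawns the Class actor at its own transform, then passes the damage to the parent implementation.
; BeginPlay, overlap and Tick are disabled stubs, and the construction script only calls the parent, so all other behavior is inherited.
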(event EventBeginPlay
  (|CallParentFunction) ; This node is disabled and will not be called.\nDrag off pins to build functionality.
)

(event Collision|EventActorBeginOverlap
  (params (OtherActor :type Actor%20Object%20Reference))
  (|CallParentFunction OtherActor) ; This node is disabled and will not be called.\nDrag off pins to build functionality.
)

(event EventTick
  (params (DeltaSeconds :type Float%20%28single-precision%29))
  (|CallParentFunction DeltaSeconds) ; This node is disabled and will not be called.\nDrag off pins to build functionality.
)

(event EventTakeDamage
  (params (damage :type Float%20%28double-precision%29))
  (Game|SpawnActorfromClass (Variables|Default|GetClass) (Transformation|GetActorTransform self) "Undefined" "MultiplyWithRoot" 0 0)
  (|CallParentFunction damage))

(fn ConstructionScript
  (|CallParentFunction))