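; BP_Shotgun is a child weapon Blueprint for the shotgun, which acts as a limited-ammo power-up for the cowboy player.
; Shoot runs the parent logic, plays a sound and decrements the ammo count (Municion).
; While ammo remains it passes the count to BP_CowBoy through UpdateShotgun; at zero it calls PowerUP(false) on the cowboy.
; Reload restores ammo to its starting value.
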(event Custom|Reload
  (Variables|Default|Setmunicion (Variables|Default|GetStartMunicion)))

(event Custom|afterShoot
  (bind _returnvalue (Game|Player|GetPlayerPawn 0))
  (bind _result (Math|Integer|DecrementInt (Variables|Default|Getmunicion))
    (:%20%20
      (bind _output_get (Variables|Default|Setmunicion _result))
      (if (<= _output_get 0)
        (bind _asbp_cow_boy (Utilities|Casting|CastToBP_CowBoy _returnvalue))
        (Default|PowerUP _asbp_cow_boy false)
        (else
          (bind _asbp_cow_boy_2 (Utilities|Casting|CastToBP_CowBoy _returnvalue))
          (Default|UpdateShotgun _asbp_cow_boy_2 _output_get))))))

(event EventBeginPlay
  (|CallParentFunction) ; This node is disabled and will not be called.\nDrag off pins to build functionality.
)

(event Collision|EventActorBeginOverlap
  (params (OtherActor :type Actor%20Object%20Reference))
  (|CallParentFunction OtherActor) ; This node is disabled and will not be called.\nDrag off pins to build functionality.
)

(event EventTick
  (params (DeltaSeconds :type Float%20%28single-precision%29))
  (|CallParentFunction DeltaSeconds) ; This node is disabled and will not be called.\nDrag off pins to build functionality.
)

(event EventShoot
  (|CallParentFunction)
  (Audio|PlaySound2D (Variables|Default|GetSound) 1.0 1.0 0.0 0 0)
  (CallFunction|AfterShoot))

(fn ConstructionScript
  (|CallParentFunction))