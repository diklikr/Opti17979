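; BP_EnemyMelee is a melee enemy that chases the player pawn in what the path names as a Wild Guns parody.
; On BeginPlay it calls MoveToPlayer, which runs AI MoveTo toward the player's current location, then binds a handler to OnFinishMove.
; A successful move calls Attack, an empty event here, and both success and failure call OnFinishMove.
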(event Custom|Attack)

(event Custom|MoveToPlayer
  ;[0.15 0.15 0.15 0.5] OnMoveFinish
  (CallFunction|Move (Transformation|GetActorLocation (Game|Player|GetPlayerPawn 0))))

(event EventBeginPlay
  ;[0.15 0.15 0.15 0.5] BeginPlay
  (|CallParentFunction)
  (CallFunction|MovetoPlayer)
  (EventDispatchers|AssignOnFinishMove (EventDispatchers|CreateEvent :!event Custom|MoveToPlayer)))

(event Collision|EventActorBeginOverlap
  (params (OtherActor :type Actor%20Object%20Reference))
  (|CallParentFunction OtherActor) ; This node is disabled and will not be called.\nDrag off pins to build functionality.
)

(event EventTick
  (params (DeltaSeconds :type Float%20%28single-precision%29))
  (|CallParentFunction DeltaSeconds) ; This node is disabled and will not be called.\nDrag off pins to build functionality.
)

(event EventMove
  (params (Destination :type Vector :default "0, 0, 0"))
  ;[0.15 0.15 0.15 0.5] Move
  (AI|AIMoveTo self (Math|Vector|MakeVector (Variables|Default|GetDestination%20X) (.y Destination) (.z Destination)) 0 2e+02 false
    (:OnSuccess
      (CallFunction|Attack))
    (:OnFail
      _))
  (Default|CallOnFinishMove))

(fn ConstructionScript
  (|CallParentFunction))